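; Game mode for a 3D platformer that tracks the respawn point and handles winning.
; On BeginPlay it stores the PlayerStart transform as the initial respawn point.
; UpdateRespawnPoint saves a new transform and checkpoint reference, first returning the previous checkpoint to normal so only the current one stays active.
; WinTheGame prints a victory message and tells the player's BP_MainCharacter to enter its celebration.
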(event `self.ReceiveBeginPlay`
  (bind _returnvalue (`GameplayStatics.GetActorOfClass` "/Script/Engine.PlayerStart"))
  (set `self.RespawnPoint` (`self.GetTransform` _returnvalue)))

(event `WinTheGame`
  (`KismetSystemLibrary.PrintString` "You Won!")
  (bind _asbp_main_character (cast `/Game/My3DPlatformer/Core/Player/BP_MainCharacter` (`GameplayStatics.GetPlayerCharacter` 0)))
  (`/Game/My3DPlatformer/Core/Player/BP_MainCharacter.EnterCelebration` _asbp_main_character))

(fn `UpdateRespawnPoint`
  (params (RespawnPoint :type "Transform Structure") (CheckPointRef :type "/Game/My3DPlatformer/Core/RespawnSystem/BP_CheckPoint Object Reference"))
  (bind _curcheckpointref (`self.CurCheckPointRef`)
    (:`then`
      (`/Game/My3DPlatformer/Core/RespawnSystem/BP_CheckPoint.ReturnToNormal` _curcheckpointref))
    (:`else`
      _))
  (set `self.RespawnPoint` RespawnPoint)
  (set `self.CurCheckPointRef` CheckPointRef))

(fn `UserConstructionScript`)