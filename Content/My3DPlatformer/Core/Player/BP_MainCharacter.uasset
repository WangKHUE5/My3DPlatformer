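; Player character Blueprint for a 3D platformer, handling movement, camera look, coin and key pickups, and a celebration state.
; Enhanced Input actions drive jumping, control-rotation-relative movement and look, with only movement gated by CanMove's character-state check.
; AddACoin updates a counter shown on a text render, while AddAKey stores keys as gameplay tags and prints them.
; EnterCelebration switches state, blocking movement, and spawns an attached Niagara effect.
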(event `self.ReceiveBeginPlay`
  (`EnhancedInputSubsystemInterface.AddMappingContext` (pcsubsystem `EnhancedInputLocalPlayerSubsystem` (`GameplayStatics.GetPlayerController` 0)) "/Game/My3DPlatformer/Input/IMC_Default.IMC_Default" 0 (struct)))

(event `EnhancedInput|/Game/My3DPlatformer/Input/Actions/IA_MoveForword`
  (params (ActionValue :type "Float (double-precision)") (ElapsedSeconds :type "Float (double-precision)") (TriggeredSeconds :type "Float (double-precision)") (InputAction :type "InputAction Object Reference" :default "/Game/My3DPlatformer/Input/Actions/IA_MoveForword.IA_MoveForword"))
  (:`Triggered`
    (if (`self.CanMove`)
      (`self.AddMovementInput` (`KismetMathLibrary.GetForwardVector` (`self.GetControlRotation`)) ActionValue))))

(event `EnhancedInput|/Game/My3DPlatformer/Input/Actions/IA_MoveRight`
  (params (ActionValue :type "Float (double-precision)") (ElapsedSeconds :type "Float (double-precision)") (TriggeredSeconds :type "Float (double-precision)") (InputAction :type "InputAction Object Reference" :default "/Game/My3DPlatformer/Input/Actions/IA_MoveRight.IA_MoveRight"))
  (:`Triggered`
    (if (`self.CanMove`)
      (`self.AddMovementInput` (`KismetMathLibrary.GetRightVector` (`self.GetControlRotation`)) ActionValue))))

(event `EnhancedInput|/Game/My3DPlatformer/Input/Actions/IA_Jump`
  (params (ActionValue :type Boolean) (ElapsedSeconds :type "Float (double-precision)") (TriggeredSeconds :type "Float (double-precision)") (InputAction :type "InputAction Object Reference" :default "/Game/My3DPlatformer/Input/Actions/IA_Jump.IA_Jump"))
  (:`Triggered`
    (`self.Jump`)))

(event `EnhancedInput|/Game/My3DPlatformer/Input/Actions/IA_Turn`
  (params (ActionValue :type "Float (double-precision)") (ElapsedSeconds :type "Float (double-precision)") (TriggeredSeconds :type "Float (double-precision)") (InputAction :type "InputAction Object Reference" :default "/Game/My3DPlatformer/Input/Actions/IA_Turn.IA_Turn"))
  (:`Triggered`
    (`self.AddControllerYawInput` ActionValue)))

(event `EnhancedInput|/Game/My3DPlatformer/Input/Actions/IA_Lookup`
  (params (ActionValue :type "Float (double-precision)") (ElapsedSeconds :type "Float (double-precision)") (TriggeredSeconds :type "Float (double-precision)") (InputAction :type "InputAction Object Reference" :default "/Game/My3DPlatformer/Input/Actions/IA_Lookup.IA_Lookup"))
  (:`Triggered`
    (`self.AddControllerPitchInput` ActionValue)))

(fn `AddACoin`
  (bind _output_get (set `self.NumCoins` (+ (`self.NumCoins`) 1)))
  (`TextRenderComponent.K2_SetText` (`self.TextRender`) (`KismetTextLibrary.Conv_IntToText` _output_get false true 2)))

(fn `AddAKey`
  (params (KeyToObtain :type "GameplayTag Structure"))
  (bind _keycollected (`self.KeyCollected`))
  (`BlueprintGameplayTagLibrary.AddGameplayTag` _keycollected KeyToObtain)
  (`KismetSystemLibrary.PrintString` (`BlueprintGameplayTagLibrary.GetDebugStringFromGameplayTagContainer` _keycollected)))

(fn `CanMove`
  (returns (ReturnValue :type Boolean))
  (return (`|EnumEquality` (`self.CharacterState`) "NewEnumerator1")))

(fn `EnterCelebration`
  (set `self.CharacterState` "NewEnumerator2")
  (`NiagaraFunctionLibrary.SpawnSystemAttached` "/Game/TeachersMarketplace/Assets/VFX/Emitters/Character/NS_Celebrate.NS_Celebrate" (`self.CapsuleComponent`) "None" (0.0 0.0 0.0) (struct) "SnapToTarget"))

(fn `UserConstructionScript`)